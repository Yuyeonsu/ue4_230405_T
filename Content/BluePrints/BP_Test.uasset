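; BP_Test is a scratch Blueprint for trying out functions, variables and debug printing.
; On BeginPlay it calls its AddNumber function, which returns the sum of two inputs, and prints the result for a pair of constants.
; A disconnected chain that increments and prints FirstNumber never runs.
; Tick, overlap and the construction script are empty.
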(event `self.ReceiveBeginPlay`
  (bind _c (`self.AddNumber` 3 5))
  (`KismetSystemLibrary.PrintString` (`KismetStringLibrary.Conv_IntToString` _c)))

(event `self.ReceiveTick`
  (params (DeltaSeconds :type "Float (single-precision)")))

(fn `AddNumber`
  (params (a :type Integer) (b :type Integer))
  (returns (c :type Integer))
  (return (+ a b)))

(fn `UserConstructionScript`)